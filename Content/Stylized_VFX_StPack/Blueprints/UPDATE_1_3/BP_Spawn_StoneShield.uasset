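; Stylized VFX pack spawner actor that repeatedly plays a stone shield Niagara effect at its own location.
; The Level variable selects one of three shield systems and staggers the first spawn after BeginPlay, with higher levels starting later.
; A custom Again event then calls itself after a fixed delay, looping the same effect indefinitely.
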(event Custom|Again
  (bind _returnvalue (Transformation|GetActorLocation))
  (Utilities|FlowControl|Delay 12.0)
  (switch int (Variables|Default|GetLevel)
    (:1
      (Niagara|SpawnSystematLocation "/Game/Stylized_VFX_StPack/Particles/UPDATE_1_3/P_StoneShield_01.P_StoneShield_01" _returnvalue))
    (:2
      (Niagara|SpawnSystematLocation "/Game/Stylized_VFX_StPack/Particles/UPDATE_1_3/P_StoneShield_02.P_StoneShield_02" _returnvalue))
    (:3
      (Niagara|SpawnSystematLocation "/Game/Stylized_VFX_StPack/Particles/UPDATE_1_3/P_StoneShield_03.P_StoneShield_03" (Transformation|GetActorLocation))))
  (CallFunction|Again))

(event EventBeginPlay
  (bind _returnvalue (Transformation|GetActorLocation))
  (Utilities|FlowControl|Delay (- (* (Variables|Default|GetLevel) 4.0) 4.0))
  (switch int (Variables|Default|GetLevel)
    (:1
      (Niagara|SpawnSystematLocation "/Game/Stylized_VFX_StPack/Particles/UPDATE_1_3/P_StoneShield_01.P_StoneShield_01" _returnvalue))
    (:2
      (Niagara|SpawnSystematLocation "/Game/Stylized_VFX_StPack/Particles/UPDATE_1_3/P_StoneShield_02.P_StoneShield_02" _returnvalue))
    (:3
      (Niagara|SpawnSystematLocation "/Game/Stylized_VFX_StPack/Particles/UPDATE_1_3/P_StoneShield_03.P_StoneShield_03" (Transformation|GetActorLocation))))
  (CallFunction|Again))

(fn ConstructionScript)