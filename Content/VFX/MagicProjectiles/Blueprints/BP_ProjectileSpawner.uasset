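; BP_ProjectileSpawner is an actor that repeatedly fires magic projectiles from its Arrow component's position.
; BeginPlay starts a looping timer at FireRate that runs the Spawn event.
; Each Spawn creates a ProjectileClass actor, ignoring collisions, and plays the MuzzleVFX system at the same location, both using the actor's rotation rather than the arrow's.
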(event Custom|Spawn
  (Game|SpawnActorfromClass (Variables|Default|GetProjectileClass) (Math|Transform|MakeTransform (Transformation|GetWorldLocation (Variables|Default|GetArrow)) (Transformation|GetActorRotation)) "AlwaysSpawn" 0 0)
  (Niagara|SpawnSystematLocation (Variables|Default|GetMuzzleVFX) (Transformation|GetWorldLocation (Variables|Default|GetArrow)) (Transformation|GetActorRotation)))

(event EventBeginPlay
  (Utilities|Time|SetTimerbyEvent (delegate Custom|Spawn) (Variables|Default|GetFireRate) true))

(fn ConstructionScript)