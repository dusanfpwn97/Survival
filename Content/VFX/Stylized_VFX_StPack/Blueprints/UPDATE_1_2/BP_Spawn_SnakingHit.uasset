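; Demo-style spawner actor that repeatedly plays a stylized snaking hit Niagara effect at its own location.
; The Level variable selects one of three effect variants and sets the initial BeginPlay delay in seconds, staggering instances of different levels.
; After each spawn, the custom Again event re-triggers itself through a fixed delay, looping the effect for as long as Level matches a variant.
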(event Custom|Again
  (bind _returnvalue (Transformation|GetActorLocation))
  (Utilities|FlowControl|Delay 3.0)
  (switch int (Variables|Default|GetLevel)
    (:1
      (Niagara|SpawnSystematLocation "/Game/VFX/Stylized_VFX_StPack/Particles/UPDATE_1_2/P_Snaking_Hit_01.P_Snaking_Hit_01" _returnvalue))
    (:2
      (Niagara|SpawnSystematLocation "/Game/VFX/Stylized_VFX_StPack/Particles/UPDATE_1_2/P_Snaking_Hit_02.P_Snaking_Hit_02" _returnvalue))
    (:3
      (Niagara|SpawnSystematLocation "/Game/VFX/Stylized_VFX_StPack/Particles/UPDATE_1_2/P_Snaking_Hit_03.P_Snaking_Hit_03" _returnvalue)))
  (CallFunction|Again))

(event EventBeginPlay
  (bind _returnvalue (Transformation|GetActorLocation))
  (Utilities|FlowControl|Delay (* (Variables|Default|GetLevel) 1.0))
  (switch int (Variables|Default|GetLevel)
    (:1
      (Niagara|SpawnSystematLocation "/Game/VFX/Stylized_VFX_StPack/Particles/UPDATE_1_2/P_Snaking_Hit_01.P_Snaking_Hit_01" _returnvalue))
    (:2
      (Niagara|SpawnSystematLocation "/Game/VFX/Stylized_VFX_StPack/Particles/UPDATE_1_2/P_Snaking_Hit_02.P_Snaking_Hit_02" _returnvalue))
    (:3
      (Niagara|SpawnSystematLocation "/Game/VFX/Stylized_VFX_StPack/Particles/UPDATE_1_2/P_Snaking_Hit_03.P_Snaking_Hit_03" _returnvalue)))
  (CallFunction|Again))

(fn ConstructionScript)