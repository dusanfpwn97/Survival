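; BP_SpawnSphericalShield is a spawner actor that repeatedly creates spherical shield VFX actors at its own location.
; From BeginPlay it loops through the Again event, spawning a new shield every eight seconds via a Delay.
; The Bv2 flag selects BP_Spherical_Shield_V2 or the original BP_Spherical_Shield.
; The spawner passes its target actor, material, particle, color, duration and scale settings to each spawned shield.
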(event Custom|Again
  (if (Variables|Default|Getbv2)
    (Game|SpawnActorfromClass "/Game/VFX/Stylized_VFX_StPack/Blueprints/BP_Spherical_Shield_V2.BP_Spherical_Shield_V2_C" (Math|Transform|MakeTransform (Transformation|GetActorLocation) "0, 0, 0" "1,1,1") "Undefined" 0 (Variables|Default|GetActor_Shield) (Variables|Default|GetMI_Shield_Material) (Variables|Default|GetParticles_Amount) (Variables|Default|GetParticles_Size) (Variables|Default|GetOutsideColor) (Variables|Default|GetInsideColor) "(R=0.786458,G=0.571834,B=0.038624,A=1.000000)" (Variables|Default|GetDuration) (Variables|Default|GetScale) 0)
    (else
      (Game|SpawnActorfromClass "/Game/VFX/Stylized_VFX_StPack/Blueprints/BP_Spherical_Shield.BP_Spherical_Shield_C" (Math|Transform|MakeTransform (Transformation|GetActorLocation) "0, 0, 0" "1,1,1") "Undefined" 0 (Variables|Default|GetMI_Shield_Material) (Variables|Default|GetParticles_Amount) (Variables|Default|GetParticles_Size) (Variables|Default|GetOutsideColor) (Variables|Default|GetInsideColor) "(R=0.786458,G=0.571834,B=0.038624,A=1.000000)" (Variables|Default|GetDuration) (Variables|Default|GetScale) true 2 false (Variables|Default|GetActor_Shield) 0)))
  (Utilities|FlowControl|Delay 8.0)
  (CallFunction|Again))

(event EventBeginPlay
  (if (Variables|Default|Getbv2)
    (Game|SpawnActorfromClass "/Game/VFX/Stylized_VFX_StPack/Blueprints/BP_Spherical_Shield_V2.BP_Spherical_Shield_V2_C" (Math|Transform|MakeTransform (Transformation|GetActorLocation) "0, 0, 0" "1,1,1") "Undefined" 0 (Variables|Default|GetActor_Shield) (Variables|Default|GetMI_Shield_Material) (Variables|Default|GetParticles_Amount) (Variables|Default|GetParticles_Size) (Variables|Default|GetOutsideColor) (Variables|Default|GetInsideColor) "(R=0.786458,G=0.571834,B=0.038624,A=1.000000)" (Variables|Default|GetDuration) (Variables|Default|GetScale) 0)
    (else
      (Game|SpawnActorfromClass "/Game/VFX/Stylized_VFX_StPack/Blueprints/BP_Spherical_Shield.BP_Spherical_Shield_C" (Math|Transform|MakeTransform (Transformation|GetActorLocation) "0, 0, 0" "1,1,1") "Undefined" 0 (Variables|Default|GetMI_Shield_Material) (Variables|Default|GetParticles_Amount) (Variables|Default|GetParticles_Size) (Variables|Default|GetOutsideColor) (Variables|Default|GetInsideColor) "(R=0.786458,G=0.571834,B=0.038624,A=1.000000)" (Variables|Default|GetDuration) (Variables|Default|GetScale) true 2 false (Variables|Default|GetActor_Shield) 0)))
  (Utilities|FlowControl|Delay 8.0)
  (CallFunction|Again))

(fn ConstructionScript)