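; BP_Missile is a VFX projectile actor that flies forward trailing smoke, then explodes and destroys itself.
; On BeginPlay it spawns the smoke system and starts the Rotation timeline, which animates the missile component's pitch and yaw while moving the actor forward without sweep and dragging the smoke along.
; When the timeline finishes, it deactivates the smoke and spawns an orange-tinted energy explosion, so detonation is timed rather than collision-driven.
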(event EventBeginPlay
  (bind _returnvalue (Transformation|GetActorLocation))
  (bind _returnvalue_2 (Niagara|SpawnSystematLocation "/Game/VFX/Stylized_VFX_StPack/Particles/UPDATE_1_4/P_Missile_Smoke.P_Missile_Smoke" "0, 0, 0"))
  (Variables|Default|SetSmoke _returnvalue_2)
  (bind (_direction _rotation_01 _rotation_02) (Timeline|Rotation PlayFromStart)
    (:Update
      (Transformation|SetWorldRotation (Variables|Components|GetMissile) (Math|Rotator|MakeRotator 0.0 _rotation_01 _rotation_02) false false)
      (Transformation|SetActorLocation (+ _returnvalue (* (Transformation|GetActorForwardVector) (* (Utilities|Time|GetWorldDeltaSeconds) 1.5e+03))) false false)
      (Transformation|SetWorldLocation (Variables|Default|GetSmoke) _returnvalue false true))
    (:Finished
      (Components|Activation|Deactivate (Variables|Default|GetSmoke))
      (bind _returnvalue_3 (Niagara|SpawnSystematLocation "/Game/VFX/Stylized_VFX_StPack/Particles/P_ExplosionEnergy_03.P_ExplosionEnergy_03" (Transformation|GetActorLocation)))
      (Effects|Components|ParticleSystem|SetColorParameter _returnvalue_3 "User.Color" "(R=0.916667,G=0.260036,B=0.000000,A=1.000000)")
      (Effects|Components|ParticleSystem|SetColorParameter _returnvalue_3 "User.SecondaryColor" "(R=1.000000,G=0.604231,B=0.000000,A=1.000000)")
      (Actor|DestroyActor))))

(fn ConstructionScript)