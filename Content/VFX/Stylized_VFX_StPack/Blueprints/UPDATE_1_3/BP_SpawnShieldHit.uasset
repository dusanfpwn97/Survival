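; Spawner actor that endlessly fires BP_Cosmic_Projectile from its own location and rotation, apparently to demo shield-hit VFX.
; BeginPlay waits for a startup delay scaled by Level, then spawns three projectiles spaced by fixed delays.
; The Again custom event loops back past the startup delay to repeat the burst, leaving a longer pause between rounds.
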(event Custom|Again
  (Utilities|FlowControl|Delay 2.0)
  (Game|SpawnActorfromClass "/Game/VFX/Stylized_VFX_StPack/Blueprints/UPDATE_1_2/BP_Cosmic_Projectile.BP_Cosmic_Projectile_C" (Math|Transform|MakeTransform (Transformation|GetActorLocation) (Transformation|GetActorRotation) "1,1,1") "Undefined" 0 false 1e+03 1 0)
  (Utilities|FlowControl|Delay 2.0)
  (Game|SpawnActorfromClass "/Game/VFX/Stylized_VFX_StPack/Blueprints/UPDATE_1_2/BP_Cosmic_Projectile.BP_Cosmic_Projectile_C" (Math|Transform|MakeTransform (Transformation|GetActorLocation) (Transformation|GetActorRotation) "1,1,1") "Undefined" 0 false 1e+03 1 0)
  (Utilities|FlowControl|Delay 2.0)
  (Game|SpawnActorfromClass "/Game/VFX/Stylized_VFX_StPack/Blueprints/UPDATE_1_2/BP_Cosmic_Projectile.BP_Cosmic_Projectile_C" (Math|Transform|MakeTransform (Transformation|GetActorLocation) (Transformation|GetActorRotation) "1,1,1") "Undefined" 0 false 1e+03 1 0)
  (Utilities|FlowControl|Delay 2.0)
  (CallFunction|Again))

(event EventBeginPlay
  (Utilities|FlowControl|Delay (* (Variables|Default|GetLevel) 0.5))
  (Utilities|FlowControl|Delay 2.0)
  (Game|SpawnActorfromClass "/Game/VFX/Stylized_VFX_StPack/Blueprints/UPDATE_1_2/BP_Cosmic_Projectile.BP_Cosmic_Projectile_C" (Math|Transform|MakeTransform (Transformation|GetActorLocation) (Transformation|GetActorRotation) "1,1,1") "Undefined" 0 false 1e+03 1 0)
  (Utilities|FlowControl|Delay 2.0)
  (Game|SpawnActorfromClass "/Game/VFX/Stylized_VFX_StPack/Blueprints/UPDATE_1_2/BP_Cosmic_Projectile.BP_Cosmic_Projectile_C" (Math|Transform|MakeTransform (Transformation|GetActorLocation) (Transformation|GetActorRotation) "1,1,1") "Undefined" 0 false 1e+03 1 0)
  (Utilities|FlowControl|Delay 2.0)
  (Game|SpawnActorfromClass "/Game/VFX/Stylized_VFX_StPack/Blueprints/UPDATE_1_2/BP_Cosmic_Projectile.BP_Cosmic_Projectile_C" (Math|Transform|MakeTransform (Transformation|GetActorLocation) (Transformation|GetActorRotation) "1,1,1") "Undefined" 0 false 1e+03 1 0)
  (Utilities|FlowControl|Delay 2.0)
  (CallFunction|Again))

(fn ConstructionScript)