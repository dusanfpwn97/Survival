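; Base Flick spell: a reusable projectile that launches from the player and homes on the closest enemy.
; Tick steers it toward its target, retargeting if lost; overlap damages living, valid actors, then resets it.
; Start, impact and damage trigger additional-projectile, explosion and bounce modifiers, with modifier instances running their own setup.
; Bounce picks the nearest enemy other than the instigator's target using a sphere nudged to refresh overlaps.
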(event OnComponentBeginOverlap(MainCollider)
  (params (OverlappedComponent :type Primitive%20Component%20Object%20Reference) (OtherActor :type Actor%20Object%20Reference) (OtherComp :type Primitive%20Component%20Object%20Reference) (OtherBodyIndex :type Integer) (bFromSweep :type Boolean) (SweepResult :type Hit%20Result%20Structure%20%28by%20ref%29))
  (if (not (Variables|Default|GetIsAvailable))
    (bind _isalive (Class|BPCombatInterface|GetIsAlive(Message) OtherActor))
    (if _isalive
      (if (CallFunction|CanDamageActor OtherActor)
        (CallFunction|DoDamage OtherActor)
        (Utilities|FlowControl|Sequence
          (:then_0
            (if (CallFunction|HasModifier "NewEnumerator5")
              (CallFunction|TriggerModifier "NewEnumerator5" self)))
          (:then_1
            (if (CallFunction|HasModifier "NewEnumerator4")
              (Utilities|FlowControl|Delay 0.1))
            (CallFunction|Reset)))))))

(event EventBeginPlay
  (|CallParentFunction))

(event EventStart
  (|CallParentFunction)
  (bind _enemy (Default|GetClosestEnemy (Variables|/Game/_Core/Spells/BP_SpellManager_Base.BP_SpellManager_Base_C|GetPlayerPawnRef (Variables|Default|GetSpellManager))))
  (Variables|Default|SetTarget _enemy)
  (Utilities|FlowControl|Sequence
    (:then_0
      (if (or (not (Variables|Default|GetIsModifier)) (CallFunction|HasModifier "NewEnumerator0"))
        (Transformation|SetActorLocation (Transformation|GetWorldLocation (Variables|/Game/_Core/BP_Player.BP_Player_C|GetSpellStart (Variables|/Game/_Core/Spells/BP_SpellManager_Base.BP_SpellManager_Base_C|GetPlayerPawnRef (Variables|Default|GetSpellManager)))) false false)
        (Utilities|IsValid (Variables|Default|GetTarget)
          (:Is%20Valid
            (bind _output_get (Variables|Default|SetStartingTargetLocation (Math|Vector|MakeVector (.x (Transformation|GetActorLocation (Variables|Default|GetTarget))) (.y (Transformation|GetActorLocation (Variables|Default|GetTarget))) (.z (Transformation|GetActorLocation (Variables|Default|GetTarget))))))
            (Variables|Default|SetStartingDirection (Math|Vector|MakeVector (.x (Math|Vector|GetForwardVector (Math|Rotator|FindLookatRotation (Transformation|GetActorLocation) _output_get))) (.y (Math|Vector|GetForwardVector (Math|Rotator|FindLookatRotation (Transformation|GetActorLocation) _output_get))) 0.0))))))
    (:then_1
      (if (not (Variables|Default|GetIsModifier))
        (if (CallFunction|HasModifier "NewEnumerator0")
          (CallFunction|TriggerModifier "NewEnumerator0" self))))
    (:then_2
      (switch Utilities|FlowControl|Switch|SwitchonE_SpellModifiers (Variables|Default|GetModifierSpell)
        (:NewEnumerator0
          (CallFunction|ActivateAdditionalProjectile))
        (:NewEnumerator4
          (CallFunction|ActivateBounce))))))

(event EventTick
  (params (DeltaSeconds :type Float%20%28single-precision%29))
  (|CallParentFunction DeltaSeconds)
  (if (not (Variables|Default|GetIsAvailable))
    (Utilities|IsValid (Variables|Default|GetTarget)
      (:Is%20Valid
        (Transformation|AddActorWorldOffset (* (Math|Vector|Normalize (- (Transformation|GetActorLocation (Variables|Default|GetTarget)) (Transformation|GetActorLocation)) 0.1) (* (Utilities|Time|GetWorldDeltaSeconds) (Variables|Default|GetSpeed))) :!label _label))
      (:Is%20Not%20Valid
        (bind _enemy (Default|GetClosestEnemy (Variables|/Game/_Core/Spells/BP_SpellManager_Base.BP_SpellManager_Base_C|GetPlayerPawnRef (Variables|Default|GetSpellManager))))
        (bind _output_get (Variables|Default|SetTarget _enemy))
        (Utilities|IsValid _output_get
          (:Is%20Valid
            (goto _label))
          (:Is%20Not%20Valid
            (CallFunction|Reset)))))))

(event Collision|EventActorBeginOverlap
  (params (OtherActor :type Actor%20Object%20Reference))
  (|CallParentFunction OtherActor) ; This node is disabled and will not be called.\nDrag off pins to build functionality.
)

(event EventDoDamage
  (params (ActorsToDamage :type Actor%20Object%20Reference))
  (|CallParentFunction ActorsToDamage)
  (if (not (Variables|Default|GetIsModifier))
    (if (CallFunction|HasModifier "NewEnumerator4")
      (CallFunction|TriggerModifier "NewEnumerator4" self))))

(fn ConstructionScript
  (|CallParentFunction))

(fn ActivateBounce
  (Transformation|SetActorLocation (Transformation|GetActorLocation (Variables|Default|GetSpellInstigator)) false false)
  (Utilities|IsValid (Variables|Default|GetBounceDetector)
    (:Is%20Valid
      _)
    (:Is%20Not%20Valid
      (bind _returnvalue (AddComponent|AddSphereComponent false))
      (Variables|Default|SetBounceDetector _returnvalue)))
  (Collision|SetCollisionEnabled (Variables|Default|GetBounceDetector) "QueryOnly")
  (Transformation|AddWorldOffset (Variables|Default|GetBounceDetector) "0.100000, 0, 0" true false) ; refresh overlap
  (for _array_element (Collision|GetOverlappingActors (Variables|Default|GetBounceDetector) "/Game/_Core/Enemies/BP_EnemyBase.BP_EnemyBase_C" :!class /Script/Engine.PrimitiveComponent)
    (if (!= _array_element (Variables|/Game/_Core/Spells/BP_SpellBase.BP_SpellBase_C|GetTarget (Variables|Default|GetSpellInstigator)))
      (Utilities|Array|Add (LocalVariables|GetNewLocalVar_0) _array_element)))
  (Collision|SetCollisionEnabled (Variables|Default|GetBounceDetector) "NoCollision")
  (bind _actor (CallFunction|GetClosestActor (LocalVariables|GetNewLocalVar_0) self))
  (Variables|Default|SetTarget _actor)
  (Utilities|IsValid (Variables|Default|GetTarget)
    (:Is%20Valid
      (Variables|Default|SetStartingTargetLocation (Math|Vector|MakeVector (.x (Transformation|GetActorLocation (Variables|Default|GetTarget))) (.y (Transformation|GetActorLocation (Variables|Default|GetTarget))) (.z (Transformation|GetActorLocation (Variables|Default|GetTarget)))))
      (Variables|Default|SetStartingDirection (Math|Vector|MakeVector (.x (Math|Vector|Normalize (- (Math|Vector|MakeVector (.x (Variables|Default|GetStartingTargetLocation)) (.y (Variables|Default|GetStartingTargetLocation)) (.z (Transformation|GetWorldLocation (Variables|/Game/_Core/BP_Player.BP_Player_C|GetSpellStart (Variables|/Game/_Core/Spells/BP_SpellManager_Base.BP_SpellManager_Base_C|GetPlayerPawnRef (Variables|Default|GetSpellManager)))))) (Transformation|GetActorLocation)))) (.y (Math|Vector|Normalize (- (Math|Vector|MakeVector (.x (Variables|Default|GetStartingTargetLocation)) (.y (Variables|Default|GetStartingTargetLocation)) (.z (Transformation|GetWorldLocation (Variables|/Game/_Core/BP_Player.BP_Player_C|GetSpellStart (Variables|/Game/_Core/Spells/BP_SpellManager_Base.BP_SpellManager_Base_C|GetPlayerPawnRef (Variables|Default|GetSpellManager)))))) (Transformation|GetActorLocation)))) 0.0)))))

(fn ActivateAdditionalProjectile
  (bind _spellmanager (Variables|Default|GetSpellManager))
  (bind _playerpawnref (Variables|/Game/_Core/Spells/BP_SpellManager_Base.BP_SpellManager_Base_C|GetPlayerPawnRef _spellmanager))
  (bind _returnvalue (Transformation|GetActorRightVector _playerpawnref))
  (bind _spellstart (Variables|/Game/_Core/BP_Player.BP_Player_C|GetSpellStart _playerpawnref))
  (bind _returnvalue_2 (Transformation|GetWorldLocation _spellstart))
  (if (Variables|Default|GetIsModifier)
    (Transformation|SetActorLocation (Variables|Default|GetSpellInstigator) (+ (* _returnvalue 35.0) _returnvalue_2) false false)
    (else
      (Transformation|SetActorLocation (+ (* _returnvalue -35.0) _returnvalue_2) false false))))