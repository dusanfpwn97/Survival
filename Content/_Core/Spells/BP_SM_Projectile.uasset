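; Spell manager for projectile spells, extending a parent spell class's CastSpell event.
; On cast it asks the player pawn for the closest enemy through an interface message and stores it as the target.
; With a valid target and spell class, it casts the projectile from the player's SpellStart component.
; A modifier adds a second cast after a short delay scaled from the spell's cooldown.
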(event EventBeginPlay
  (|CallParentFunction) ; This node is disabled and will not be called.\nDrag off pins to build functionality.
)

(event EventTick
  (params (DeltaSeconds :type Float%20%28single-precision%29))
  (|CallParentFunction DeltaSeconds) ; This node is disabled and will not be called.\nDrag off pins to build functionality.
)

(event EventCastSpell
  (bind _playerpawnref (Variables|Default|GetPlayerPawnRef))
  (bind _spelltospawn (Variables|Default|GetSpellToSpawn))
  (bind _spellstart (Variables|/Game/_Core/BP_Player.BP_Player_C|GetSpellStart _playerpawnref))
  (bind _returnvalue (Transformation|GetWorldLocation _spellstart))
  (|CallParentFunction)
  (bind _enemy (Class|BPCombatInterface|GetClosestEnemy(Message) (Game|Player|GetPlayerPawn 0)))
  (bind _output_get (Variables|Default|SetTarget _enemy))
  (Utilities|IsValid _output_get
    (:Is%20Valid
      (if (Utilities|IsValidClass _spelltospawn)
        (CallFunction|CastASpell _spelltospawn _returnvalue)
        (if (CallFunction|HasModifier "NewEnumerator3")
          (Utilities|FlowControl|Delay (/ (.cooldown (Variables|Default|GetSpellTypeInfo)) 8.0))
          (CallFunction|CastASpell (Variables|Default|GetSpellToSpawn) _returnvalue))
        (else
          (Development|PrintString (Utilities|String|Append "CLASS NOT VALID> PROJECTILE MANAGER - " (Utilities|String|ToString(Text) (.name (Variables|Default|GetSpellTypeInfo))))))))))