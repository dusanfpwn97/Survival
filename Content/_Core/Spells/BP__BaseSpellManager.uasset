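; Base spell manager that auto-casts a projectile at the player's closest enemy whenever its cooldown expires.
; Tick drives the countdown, and each cast spawns a BP_SpellProjectile just off the player toward the target, passing target and element.
; Modifiers are stored by inventory slot after a GameInstance cast-type compatibility check, returning replaced ones to the player and refreshing the HUD.
; The two inventory getter functions are empty stubs.
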(event Custom|AddSpellModifier
  (params (InventoryIndex :type Integer) (SpellModifier :type E_SpellModifiers%20Enum :default "NewEnumerator0"))
  (bind _spellmodifiers (Variables|Default|GetSpellModifiers))
  (bind (_value _returnvalue) (Utilities|Map|Find _spellmodifiers InventoryIndex))
  (if (CallFunction|CanModifySpell SpellModifier)
    (if _returnvalue
      (Utilities|FlowControl|Sequence
        (:then_0
          (Development|PrintString (Utilities|String|Append (Utilities|String|EnumtoString SpellModifier) " Modifier already exists at this slot. Replacing..." (Utilities|GetDisplayName self)) true true "(R=1.000000,G=0.750000,B=0.000000,A=1.000000)" 3.0)
          (bind _asbp_player (Utilities|Casting|CastToBP_Player (Game|Player|GetPlayerPawn 0)))
          (Default|AddModifiertoInventory _asbp_player _value))
        (:then_1
          (Utilities|Map|Add (Variables|Default|GetSpellModifiers) InventoryIndex SpellModifier :!label _label)
          (Class|BPHUDInterface|RefreshInventory(Message) (HUD|GetHUD (Game|GetPlayerController 0)))))
      (else
        (goto _label)))
    (else
      (Development|PrintString (Utilities|String|Append (Utilities|String|EnumtoString SpellModifier) " not compatible with " (Utilities|String|EnumtoString (Variables|Default|GetSpellCastType)) "! " (Utilities|GetDisplayName self)) true true "(R=1.000000,G=0.182798,B=0.000000,A=1.000000)" 5.0))))

(event Custom|UpdateManager
  (if (<= (- (Variables|Default|GetCurrentCooldown) (Utilities|Time|GetWorldDeltaSeconds)) 0.0)
    (Variables|Default|SetCurrentCooldown (Variables|Default|GetCooldown))
    (CallFunction|CastSpell)
    (Development|PrintString "Hello")
    (else
      (Variables|Default|SetCurrentCooldown (- (Variables|Default|GetCurrentCooldown) (Utilities|Time|GetWorldDeltaSeconds))))))

(event Custom|CastSpell
  (bind _returnvalue (Game|Player|GetPlayerPawn 0))
  (bind _enemy (Class|BPCombatInterface|GetClosestEnemy(Message) _returnvalue))
  (bind _output_get (Variables|Default|SetTarget _enemy))
  (Utilities|IsValid _output_get
    (:Is%20Valid
      (Game|SpawnActorfromClass "/Game/_Core/Spells/Spells/BP_SpellProjectile.BP_SpellProjectile_C" (Math|Transform|MakeTransform (Math|Vector|MakeVector (.x (+ (* (Math|Vector|GetForwardVector (Math|Rotator|FindLookatRotation (Transformation|GetActorLocation _returnvalue) (Transformation|GetActorLocation (Variables|Default|GetTarget)))) 3e+01) (Transformation|GetActorLocation (Game|Player|GetPlayerPawn 0)))) (.y (+ (* (Math|Vector|GetForwardVector (Math|Rotator|FindLookatRotation (Transformation|GetActorLocation _returnvalue) (Transformation|GetActorLocation (Variables|Default|GetTarget)))) 3e+01) (Transformation|GetActorLocation (Game|Player|GetPlayerPawn 0)))) 0.0) "0, 0, 0" "1,1,1") "Undefined" 0 (Variables|Default|GetTarget) (Variables|Default|GetElement) 0))))

(event EventBeginPlay)

(event EventTick
  (params (DeltaSeconds :type Float%20%28single-precision%29))
  (CallFunction|UpdateManager))

(event EventOnModifiedSpell
  (params (Spell :type BP%20Base%20Spell%20Manager%20Object%20Reference) (UpgradeUsed :type BP%20Drop%20Base%20Object%20Reference) (InventoryIndex :type Integer))
  (CallFunction|AddSpellModifier InventoryIndex (Variables|/Game/_Core/Drop/BP_DropBase.BP_DropBase_C|GetSpellModifier UpgradeUsed)))

(fn CanModifySpell
  (params (SpellModifier :type E_SpellModifiers%20Enum :default "NewEnumerator9"))
  (bind _compatiblemodifiers (Class|BPGameSettingsInterface|GetCompatiblesforCastType(Message) (Game|GetGameInstance) (Variables|Default|GetSpellCastType)))
  (return (Utilities|Array|ContainsItem _compatiblemodifiers SpellModifier)))

(fn GetSpellsinInventory
  (return 0))

(fn GetUpgradesinInventory
  (params (SpecificUpgrade :type E_AllUpgradeTypes%20Enum :default "NewEnumerator5"))
  (return 0))