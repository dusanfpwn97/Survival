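; Base spell manager that automatically casts a spell projectile whenever its cooldown runs out.
; Tick counts down the cooldown, then asks the player pawn for its closest enemy via an interface message.
; If that enemy is valid, it spawns BP_SpellProjectile slightly offset from the player toward it, passing target and element.
; AddSpellModifier stores unique modifiers that the GameInstance lists as compatible with the cast type, printing otherwise.
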(event Custom|AddSpellModifier
  (params (SpellModifier :type E_SpellModifiers%20Enum :default "NewEnumerator0"))
  (bind _spellcasttype (Variables|Default|GetSpellCastType))
  (bind _compatiblemodifiers (Class|BPGameSettingsInterface|GetCompatiblesforCastType(Message) (Game|GetGameInstance) (Variables|Default|GetSpellCastType)))
  (if (Utilities|Array|ContainsItem _compatiblemodifiers SpellModifier)
    (if (Utilities|Array|ContainsItem (Variables|Default|GetSpellModifiers) SpellModifier)
      (Development|PrintString (Utilities|String|Append (Utilities|String|EnumtoString SpellModifier) " Modifier already exists! " (Utilities|GetDisplayName self)) true true "(R=1.000000,G=0.182798,B=0.000000,A=1.000000)" 5.0)
      (else
        (Utilities|Array|Add (Variables|Default|GetSpellModifiers) SpellModifier)))
    (else
      (Development|PrintString (Utilities|String|Append (Utilities|String|EnumtoString _spellcasttype) " not compatible with " (Utilities|String|EnumtoString _spellcasttype) "! " (Utilities|GetDisplayName self)) true true "(R=1.000000,G=0.182798,B=0.000000,A=1.000000)" 5.0))))

(event Custom|UpdateManager
  (if (<= (- (Variables|Default|GetCurrentCooldown) (Utilities|Time|GetWorldDeltaSeconds)) 0.0)
    (Variables|Default|SetCurrentCooldown (Variables|Default|GetCooldown))
    (CallFunction|CastSpell)
    (else
      (Variables|Default|SetCurrentCooldown (- (Variables|Default|GetCurrentCooldown) (Utilities|Time|GetWorldDeltaSeconds))))))

(event Custom|CastSpell
  (bind _returnvalue (Game|Player|GetPlayerPawn 0))
  (bind _enemy (Class|BPCombatInterface|GetClosestEnemy(Message) _returnvalue))
  (bind _output_get (Variables|Default|SetTarget _enemy))
  (Utilities|IsValid _output_get
    (:Is%20Valid
      (Game|SpawnActorfromClass "/Game/_Core/Spells/Spells/BP_SpellProjectile.BP_SpellProjectile_C" (Math|Transform|MakeTransform (Math|Vector|MakeVector (.x (+ (* (Math|Vector|GetForwardVector (Math|Rotator|FindLookatRotation (Transformation|GetActorLocation _returnvalue) (Transformation|GetActorLocation (Variables|Default|GetTarget)))) 3e+01) (Transformation|GetActorLocation (Game|Player|GetPlayerPawn 0)))) (.y (+ (* (Math|Vector|GetForwardVector (Math|Rotator|FindLookatRotation (Transformation|GetActorLocation _returnvalue) (Transformation|GetActorLocation (Variables|Default|GetTarget)))) 3e+01) (Transformation|GetActorLocation (Game|Player|GetPlayerPawn 0)))) 0.0) "0, 0, 0" "1,1,1") "Undefined" 0 (Variables|Default|GetTarget) (Variables|Default|GetElement) 0))))

(event EventBeginPlay)

(event EventTick
  (params (DeltaSeconds :type Float%20%28single-precision%29))
  (CallFunction|UpdateManager))