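; Spell manager for the Flick spell, which casts a projectile when the player pawn reports a closest enemy.
; On CastSpell it stores that enemy as Target and, if valid, casts the configured spell class from the pawn's SpellStart point.
; A specific modifier adds a second cast after one eighth of the spell's cooldown.
; An unset spell class prints an error with the spell name.
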(event EventBeginPlay
  (|CallParentFunction) ; This node is disabled and will not be called.\nDrag off pins to build functionality.
)

(event EventTick
  (params (DeltaSeconds :type Float%20%28single-precision%29))
  (|CallParentFunction DeltaSeconds) ; This node is disabled and will not be called.\nDrag off pins to build functionality.
)

(event EventCastSpell
  (bind _spelltospawn (Variables|Default|GetSpellToSpawn))
  (|CallParentFunction)
  (bind _enemy (Class|BPCombatInterface|GetClosestEnemy(Message) (Game|Player|GetPlayerPawn 0)))
  (bind _output_get (Variables|Default|SetTarget _enemy))
  (Utilities|IsValid _output_get
    (:Is%20Valid
      (if (Utilities|IsValidClass _spelltospawn)
        (CallFunction|CastASpell _spelltospawn (Transformation|GetWorldLocation (Variables|/Game/_Core/BP_Player.BP_Player_C|GetSpellStart (Variables|Default|GetPlayerPawnRef))))
        (if (CallFunction|HasModifier "NewEnumerator3")
          (Utilities|FlowControl|Delay (/ (.cooldown (Variables|Default|GetSpellTypeInfo)) 8.0))
          (CallFunction|CastASpell (Variables|Default|GetSpellToSpawn) (Transformation|GetWorldLocation (Variables|/Game/_Core/BP_Player.BP_Player_C|GetSpellStart (Variables|Default|GetPlayerPawnRef)))))
        (else
          (Development|PrintString (Utilities|String|Append "CLASS NOT VALID> PROJECTILE MANAGER - " (Utilities|String|ToString(Text) (.name (Variables|Default|GetSpellTypeInfo))))))))))