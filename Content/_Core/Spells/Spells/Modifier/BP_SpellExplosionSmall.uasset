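; BP_SpellExplosionSmall is a small explosion spell in the modifier group that deals area damage to enemies.
; On Start it runs the parent logic, then passes every BP_EnemyBase actor overlapping its main collider to DoDamageMultiple in a single hit.
; After a short delay it calls Reset, leaving all other behavior to its parent class.
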(event EventBeginPlay
  (|CallParentFunction))

(event EventStart
  (|CallParentFunction)
  (CallFunction|DoDamageMultiple (Collision|GetOverlappingActors (Variables|Default|GetMainCollider) "/Game/_Core/Enemies/BP_EnemyBase.BP_EnemyBase_C" :!class /Script/Engine.PrimitiveComponent))
  (Utilities|FlowControl|Delay 2.0)
  (CallFunction|Reset))

(event EventTick
  (params (DeltaSeconds :type Float%20%28single-precision%29))
  (|CallParentFunction DeltaSeconds))

(fn ConstructionScript
  (|CallParentFunction))