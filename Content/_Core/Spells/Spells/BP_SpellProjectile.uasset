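; BP_SpellProjectile is a spell projectile that flies in a straight line and damages actors it overlaps.
; Init picks the main Niagara effect from the spell's Element, printing an error when none is set.
; Tick moves it along StartingDirection by Speed without sweeping, so hits rely on the collider overlap.
; An overlap applies fixed damage regardless of element and destroys the projectile, which otherwise expires after a short lifetime.
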(event OnComponentBeginOverlap(MainCollider)
  (params (OverlappedComponent :type Primitive%20Component%20Object%20Reference) (OtherActor :type Actor%20Object%20Reference) (OtherComp :type Primitive%20Component%20Object%20Reference) (OtherBodyIndex :type Integer) (bFromSweep :type Boolean) (SweepResult :type Hit%20Result%20Structure%20%28by%20ref%29))
  (Game|Damage|ApplyDamage OtherActor 1e+02 0 0)
  (Utilities|FlowControl|Delay 0.0)
  (Actor|DestroyActor))

(event EventBeginPlay
  (|CallParentFunction)
  (Utilities|FlowControl|Delay 5.0)
  (Actor|DestroyActor))

(event EventTick
  (params (DeltaSeconds :type Float%20%28single-precision%29))
  (|CallParentFunction DeltaSeconds)
  (Transformation|AddActorWorldOffset (* (Variables|Default|GetStartingDirection) (* (Utilities|Time|GetWorldDeltaSeconds) (Variables|Default|GetSpeed)))))

(event EventInit
  (bind _mainngsystem (Variables|Default|GetMainNGSystem))
  (|CallParentFunction)
  (switch Utilities|FlowControl|Switch|SwitchonE_Elements (Variables|Default|GetElement)
    (:NewEnumerator9
      (Development|PrintString (Utilities|String|Append "Init Spell Has no Element set! " (Utilities|GetDisplayName self)) true true "(R=1.000000,G=0.041237,B=0.000000,A=1.000000)"))
    (:NewEnumerator0
      (Class|NiagaraComponent|SetAsset _mainngsystem "/Game/Particles/Projectiles/NS_FireProjectile.NS_FireProjectile"))
    (:NewEnumerator1
      (Class|NiagaraComponent|SetAsset _mainngsystem "/Game/Particles/Projectiles/NS_WaterProjectile.NS_WaterProjectile"))
    (:NewEnumerator2
      (Class|NiagaraComponent|SetAsset _mainngsystem "/Game/Particles/Projectiles/NS_WindProjectile.NS_WindProjectile"))
    (:NewEnumerator3
      (Class|NiagaraComponent|SetAsset _mainngsystem "/Game/Particles/Projectiles/NS_ElectricProjectile.NS_ElectricProjectile"))
    (:NewEnumerator4
      (Class|NiagaraComponent|SetAsset _mainngsystem "/Game/Particles/Projectiles/NS_PoisonProjectile.NS_PoisonProjectile"))
    (:NewEnumerator5
      (Class|NiagaraComponent|SetAsset _mainngsystem "/Game/Particles/Projectiles/NS_DarkProjectile.NS_DarkProjectile"))
    (:NewEnumerator6
      (Class|NiagaraComponent|SetAsset _mainngsystem "/Game/Particles/Projectiles/NS_EarthProjectile.NS_EarthProjectile"))))

(fn ConstructionScript
  (|CallParentFunction))