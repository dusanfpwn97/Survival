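; BP_SpellBaseProjectile is a base projectile spell that flies in a straight line and damages what it hits.
; Tick offsets the actor along StartingDirection by Speed and world delta time, without sweeping.
; While active, MainCollider overlaps pass alive and CanDamageActor checks before calling DoDamage, which defers to the parent.
; Modifier-based hit-count and reset logic remains in the graph but is disconnected.
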(event OnComponentBeginOverlap(MainCollider)
  (params (OverlappedComponent :type Primitive%20Component%20Object%20Reference) (OtherActor :type Actor%20Object%20Reference) (OtherComp :type Primitive%20Component%20Object%20Reference) (OtherBodyIndex :type Integer) (bFromSweep :type Boolean) (SweepResult :type Hit%20Result%20Structure%20%28by%20ref%29))
  (if (Variables|Default|GetIsActive)
    (bind _isalive (Class|BPCombatInterface|GetIsAlive(Message) OtherActor))
    (if _isalive
      (if (CallFunction|CanDamageActor OtherActor)
        (CallFunction|DoDamage OtherActor)))))

(event EventBeginPlay
  (|CallParentFunction))

(event EventTick
  (params (DeltaSeconds :type Float%20%28single-precision%29))
  (|CallParentFunction DeltaSeconds)
  (Transformation|AddActorWorldOffset (* (Variables|Default|GetStartingDirection) (* (Utilities|Time|GetWorldDeltaSeconds) (Variables|Default|GetSpeed)))))

(event Collision|EventActorBeginOverlap
  (params (OtherActor :type Actor%20Object%20Reference))
  (|CallParentFunction OtherActor) ; This node is disabled and will not be called.\nDrag off pins to build functionality.
)

(event EventDoDamage
  (params (ActorsToDamage :type Actor%20Object%20Reference))
  (|CallParentFunction ActorsToDamage))

(fn ConstructionScript
  (|CallParentFunction))