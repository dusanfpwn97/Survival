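; Small explosion spell Blueprint in the modifier spells set that deals instant area damage.
; On InitSpell it re-sets its actor location to the current one, then calls DoDamage once on every actor overlapping MainCollider.
; BeginPlay, Tick and construction only pass through to the parent class.
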(event EventBeginPlay
  (|CallParentFunction))

(event EventInitSpell
  (params (IsModifier :type Boolean) (TargetEnemy :type Object%20Object%20Reference) (StartLocation :type Vector :default "0, 0, 0"))
  (Transformation|SetActorLocation (Transformation|GetActorLocation) false false)
  (for _array_element (Collision|GetOverlappingActors (Variables|Default|GetMainCollider) 0 :!class /Script/Engine.PrimitiveComponent)
    (CallFunction|DoDamage _array_element)))

(event EventTick
  (params (DeltaSeconds :type Float%20%28single-precision%29))
  (|CallParentFunction DeltaSeconds))

(fn ConstructionScript
  (|CallParentFunction))