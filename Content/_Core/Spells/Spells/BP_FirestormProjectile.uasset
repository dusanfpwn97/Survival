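; Firestorm spell projectile that falls diagonally and explodes on overlap.
; Tick moves it by a fixed horizontal drift plus a Speed-driven descent, scaled by delta time.
; MainCollider overlap applies fixed damage to the other actor, spawns a pooled Niagara explosion and destroys the projectile after a short delay.
; BeginPlay sets a timed self-destruct; its Speed randomization runs only after DestroyActor, so it never affects the fall.
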(event OnComponentBeginOverlap(MainCollider)
  (params (OverlappedComponent :type Primitive%20Component%20Object%20Reference) (OtherActor :type Actor%20Object%20Reference) (OtherComp :type Primitive%20Component%20Object%20Reference) (OtherBodyIndex :type Integer) (bFromSweep :type Boolean) (SweepResult :type Hit%20Result%20Structure%20%28by%20ref%29))
  (Game|Damage|ApplyDamage OtherActor 1e+02 0 0)
  (Niagara|SpawnSystematLocation "/Game/Particles/Projectiles/NS_FirestormProjectileExplode.NS_FirestormProjectileExplode" (Transformation|GetActorLocation) "0, 0, 0" "1.000000,1.000000,1.000000" true true "AutoRelease")
  (Utilities|FlowControl|Delay 0.2)
  (Actor|DestroyActor))

(event Custom|Init_1)

(event EventBeginPlay
  (|CallParentFunction)
  (Utilities|FlowControl|Delay 5.0)
  (Actor|DestroyActor)
  (Variables|Default|SetSpeed (* (Variables|Default|GetSpeed) (Math|Random|RandomFloatinRange 0.8 1.2))))

(event EventTick
  (params (DeltaSeconds :type Float%20%28single-precision%29))
  (bind _returnvalue (Utilities|Time|GetWorldDeltaSeconds))
  (bind _returnvalue_2 (* _returnvalue -2e+02))
  (|CallParentFunction DeltaSeconds)
  (Transformation|AddActorWorldOffset (Math|Vector|MakeVector (* _returnvalue_2 -1.0) _returnvalue_2 (* _returnvalue (Variables|Default|GetSpeed) -1.0))))

(fn ConstructionScript
  (|CallParentFunction))