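; Base flick spell: a projectile that, while active, homes on its target or flies along its starting direction when no valid target exists.
; Tick moves it by Speed without sweeping, and DoDamage calls the parent, then resets the spell.
; The overlap handler, ActivateBounce and ActivateAdditionalProjectile do nothing; their damage check, nearest-actor retargeting and side-offset spawn logic sit disconnected and never run.
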(event OnComponentBeginOverlap(MainCollider)
  (params (OverlappedComponent :type Primitive%20Component%20Object%20Reference) (OtherActor :type Actor%20Object%20Reference) (OtherComp :type Primitive%20Component%20Object%20Reference) (OtherBodyIndex :type Integer) (bFromSweep :type Boolean) (SweepResult :type Hit%20Result%20Structure%20%28by%20ref%29))
  (if (Variables|Default|GetIsActive)
    _))

(event EventBeginPlay
  (|CallParentFunction))

(event EventTick
  (params (DeltaSeconds :type Float%20%28single-precision%29))
  (bind _returnvalue (Utilities|Time|GetWorldDeltaSeconds))
  (bind _speed (Variables|Default|GetSpeed))
  (bind _target (Variables|Default|GetTarget))
  (bind _returnvalue_2 (* _returnvalue _speed))
  (|CallParentFunction DeltaSeconds)
  (if (Variables|Default|GetIsActive)
    (Utilities|IsValid _target
      (:Is%20Valid
        (Transformation|AddActorWorldOffset (* (Math|Vector|Normalize (- (Transformation|GetActorLocation _target) (Transformation|GetActorLocation)) 0.01) _returnvalue_2)))
      (:Is%20Not%20Valid
        (Transformation|AddActorWorldOffset (* (Variables|Default|GetStartingDirection) _returnvalue_2))))))

(event EventDoDamage
  (params (ActorsToDamage :type Actor%20Object%20Reference))
  (|CallParentFunction ActorsToDamage)
  (CallFunction|ResetSpell))

(fn ConstructionScript
  (|CallParentFunction))

(fn ActivateBounce)

(fn ActivateAdditionalProjectile)