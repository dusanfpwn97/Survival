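; BP_Projectile is a spell cast type: a projectile that flies in a straight line and destroys itself five seconds after BeginPlay.
; Tick offsets it along StartingDirection by Speed and delta time, without sweeping.
; Init calls its parent, then assigns MainNGSystem the Niagara effect matching its Element.
; The construction script calls Init only when the platform is Windows, and this Blueprint has no active overlap logic.
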(event EventBeginPlay
  (|CallParentFunction)
  (Utilities|FlowControl|Delay 5.0)
  (Actor|DestroyActor))

(event Collision|EventActorBeginOverlap
  (params (OtherActor :type Actor%20Object%20Reference))
  (|CallParentFunction OtherActor) ; This node is disabled and will not be called.\nDrag off pins to build functionality.
)

(event EventTick
  (params (DeltaSeconds :type Float%20%28single-precision%29))
  (|CallParentFunction DeltaSeconds)
  (Transformation|AddActorWorldOffset (* (Variables|Default|GetStartingDirection) (* (Utilities|Time|GetWorldDeltaSeconds) (Variables|Default|GetSpeed)))))

(event EventInit
  (bind _mainngsystem (Variables|Default|GetMainNGSystem))
  (|CallParentFunction)
  (switch Utilities|FlowControl|Switch|SwitchonE_Elements (Variables|Default|GetElement)
    (:NewEnumerator0
      (Class|NiagaraComponent|SetAsset _mainngsystem "/Game/Particles/Projectiles/NS_FireProjectile.NS_FireProjectile"))
    (:NewEnumerator1
      (Class|NiagaraComponent|SetAsset _mainngsystem "/Game/Particles/Projectiles/NS_WaterProjectile.NS_WaterProjectile"))
    (:NewEnumerator2
      (Class|NiagaraComponent|SetAsset _mainngsystem "/Game/Particles/Projectiles/NS_WindProjectile.NS_WindProjectile"))
    (:NewEnumerator3
      (Class|NiagaraComponent|SetAsset _mainngsystem "/Game/Particles/Projectiles/NS_ElectricProjectile.NS_ElectricProjectile"))
    (:NewEnumerator4
      (Class|NiagaraComponent|SetAsset _mainngsystem "/Game/Particles/Projectiles/NS_PoisonProjectile.NS_PoisonProjectile"))
    (:NewEnumerator5
      (Class|NiagaraComponent|SetAsset _mainngsystem "/Game/Particles/Projectiles/NS_DarkProjectile.NS_DarkProjectile"))
    (:NewEnumerator6
      (Class|NiagaraComponent|SetAsset _mainngsystem "/Game/Particles/Projectiles/NS_EarthProjectile.NS_EarthProjectile"))))

(fn ConstructionScript
  (|CallParentFunction)
  (if (Utilities|Enum|Equal(Enum) (Game|GetPlatformName) "Windows")
    (CallFunction|Init)))