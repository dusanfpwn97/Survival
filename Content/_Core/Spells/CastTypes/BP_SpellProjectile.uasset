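; Projectile spell cast type that flies in a straight line, with a Niagara effect chosen by its element.
; CastSpell spawns another instance of this class just off the player toward the closest enemy, passing Target and Element.
; Tick moves it along StartingDirection at Speed without sweeping, and it destroys itself after a short lifetime.
; Inventory copies stay hidden and stationary, and skip the timed destruction.
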(event EventBeginPlay
  (|CallParentFunction)
  (if (Variables|Default|GetIsForInventory)
    (Rendering|SetActorHiddenInGame true)
    (else
      (Utilities|FlowControl|Delay 5.0)
      (Actor|DestroyActor))))

(event EventTick
  (params (DeltaSeconds :type Float%20%28single-precision%29))
  (|CallParentFunction DeltaSeconds)
  (if (not (Variables|Default|GetIsForInventory))
    (Transformation|AddActorWorldOffset (* (Variables|Default|GetStartingDirection) (* (Utilities|Time|GetWorldDeltaSeconds) (Variables|Default|GetSpeed))))))

(event EventInit
  (bind _mainngsystem (Variables|Default|GetMainNGSystem))
  (|CallParentFunction)
  (switch Utilities|FlowControl|Switch|SwitchonE_Elements (Variables|Default|GetElement)
    (:NewEnumerator9
      (Development|PrintString (Utilities|String|Append "Init Spell NULL! " (Utilities|GetDisplayName self)) true true "(R=1.000000,G=0.041237,B=0.000000,A=1.000000)"))
    (:NewEnumerator0
      (Class|NiagaraComponent|SetAsset _mainngsystem "/Game/Particles/Projectiles/NS_FireProjectile.NS_FireProjectile"))
    (:NewEnumerator1
      (Class|NiagaraComponent|SetAsset _mainngsystem "/Game/Particles/Projectiles/NS_WaterProjectile.NS_WaterProjectile"))
    (:NewEnumerator2
      (Class|NiagaraComponent|SetAsset _mainngsystem "/Game/Particles/Projectiles/NS_WindProjectile.NS_WindProjectile"))
    (:NewEnumerator3
      (Class|NiagaraComponent|SetAsset _mainngsystem "/Game/Particles/Projectiles/NS_ElectricProjectile.NS_ElectricProjectile"))
    (:NewEnumerator4
      (Class|NiagaraComponent|SetAsset _mainngsystem "/Game/Particles/Projectiles/NS_PoisonProjectile.NS_PoisonProjectile"))
    (:NewEnumerator5
      (Class|NiagaraComponent|SetAsset _mainngsystem "/Game/Particles/Projectiles/NS_DarkProjectile.NS_DarkProjectile"))
    (:NewEnumerator6
      (Class|NiagaraComponent|SetAsset _mainngsystem "/Game/Particles/Projectiles/NS_EarthProjectile.NS_EarthProjectile"))))

(event EventCastSpell
  (|CallParentFunction)
  (bind _enemy (Class|BPCombatInterface|GetClosestEnemy(Message) (Game|Player|GetPlayerPawn 0)))
  (bind _output_get (Variables|Default|SetTarget _enemy))
  (Utilities|IsValid _output_get
    (:Is%20Valid
      (Game|SpawnActorfromClass "BP_SpellProjectile_C" (Math|Transform|MakeTransform (Math|Vector|MakeVector (.x (+ (* (Math|Vector|GetForwardVector (Math|Rotator|FindLookatRotation (Transformation|GetActorLocation) (Transformation|GetActorLocation (Variables|Default|GetTarget)))) 3e+01) (Transformation|GetActorLocation (Game|Player|GetPlayerPawn 0)))) (.y (+ (* (Math|Vector|GetForwardVector (Math|Rotator|FindLookatRotation (Transformation|GetActorLocation) (Transformation|GetActorLocation (Variables|Default|GetTarget)))) 3e+01) (Transformation|GetActorLocation (Game|Player|GetPlayerPawn 0)))) 0.0) "0, 0, 0" "1,1,1") "Undefined" 0 (Variables|Default|GetTarget) (Variables|Default|GetElement) false 0))))

(fn ConstructionScript
  (|CallParentFunction))