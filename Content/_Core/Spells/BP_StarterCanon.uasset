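; Starter cannon spell projectile that flies in a straight line toward where its Target stood when it spawned.
; BeginPlay stores the normalized direction to the Target once, so the shot does not home, and starts a five-second delay before destroying itself.
; Tick moves the actor along that direction by Speed and delta time, without sweeping.
; No hit or damage logic appears in these graphs.
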(event EventBeginPlay
  (|CallParentFunction)
  (Utilities|FlowControl|Sequence
    (:then_0
      (Utilities|FlowControl|Delay 5.0)
      (Actor|DestroyActor))
    (:then_1
      (Variables|Default|SetStartingTargetLocation (Transformation|GetActorLocation (Variables|Default|GetTarget)))
      (Variables|Default|SetStartingDirection (Math|Vector|Normalize (- (Variables|Default|GetStartingTargetLocation) (Transformation|GetActorLocation)))))))

(event EventTick
  (params (DeltaSeconds :type Float%20%28single-precision%29))
  (|CallParentFunction DeltaSeconds)
  (Transformation|AddActorWorldOffset (* (Variables|Default|GetStartingDirection) (* (Utilities|Time|GetWorldDeltaSeconds) (Variables|Default|GetSpeed)))))

(fn ConstructionScript
  (|CallParentFunction))