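; BP_SpellBase is a reusable spell actor base that damages actors through OnDamagedMessage and spawns modifier spells.
; Start and Reset toggle visibility, Niagara effect and availability, with a failsafe timer forcing reset.
; TriggerModifier spawns one spell per modifier type, caches it in a pool and restarts it later, blocking chaining from modifier spells except Explode on Impact.
; GetClosestEnemy, Stop and Tick are empty.
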(event Custom|DoDamage
  (params (ActorsToDamage :type Actor%20Object%20Reference))
  (Class|BPCombatInterface|OnDamaged(Message) ActorsToDamage self)
  (Math|Integer|IncrementInt (Variables|Default|GetDidDamageCount)))

(event Custom|Reset
  (bind _failsafetimerhandle (Variables|Default|GetFailsafeTimerHandle))
  (Variables|Default|SetIsAvailable true)
  (Rendering|SetActorHiddenInGame true)
  (if (Utilities|Time|IsValidTimerHandle _failsafetimerhandle)
    (Utilities|Time|ClearandInvalidateTimerbyHandle _failsafetimerhandle))
  (Class|NiagaraComponent|SetPaused (Variables|Default|GetMainNGSystem) true)
  (Variables|Default|SetDidDamageCount 0))

(event Custom|Start
  (bind _mainngsystem (Variables|Default|GetMainNGSystem))
  (Variables|Default|SetIsAvailable false)
  (Variables|Default|SetTarget 0)
  (Rendering|SetActorHiddenInGame false)
  (bind _returnvalue (Utilities|Time|SetTimerbyFunctionName 0 "Reset" (Variables|Default|GetFailsafeTimer)))
  (Variables|Default|SetFailsafeTimerHandle _returnvalue)
  (Class|NiagaraComponent|SetPaused _mainngsystem false)
  (Niagara|ReinitializeSystem _mainngsystem))

(event Custom|Stop)

(event EventBeginPlay
  (CallFunction|Reset))

(event Collision|EventActorBeginOverlap
  (params (OtherActor :type Actor%20Object%20Reference)))

(event EventTick
  (params (DeltaSeconds :type Float%20%28single-precision%29)))

(fn ConstructionScript)

(fn HasModifier
  (params (Modifier :type E_SpellModifiers%20Enum :default "NewEnumerator9"))
  (bind _values (Utilities|Map|Values (Variables|/Game/_Core/Spells/BP_SpellManager_Base.BP_SpellManager_Base_C|GetCurrentModifiers (Variables|Default|GetSpellManager))))
  (return (Utilities|Array|ContainsItem _values Modifier)))

(fn GetModiferSpellClass
  (params (Modifier :type E_SpellModifiers%20Enum :default "NewEnumerator9") (ModifiedSpell :type BP%20Spell%20Base%20Object%20Reference))
  (switch Utilities|FlowControl|Switch|SwitchonE_SpellModifiers Modifier
    (:NewEnumerator0
      _)
    (:NewEnumerator4
      _)
    (:NewEnumerator5
      (return "/Game/_Core/Spells/Spells/Modifier/BP_SpellExplosionSmall.BP_SpellExplosionSmall_C" (Transformation|GetActorLocation ModifiedSpell))))
  (return (Utilities|GetClass self) (Transformation|GetWorldLocation (Variables|/Game/_Core/BP_Player.BP_Player_C|GetSpellStart (Variables|/Game/_Core/Spells/BP_SpellManager_Base.BP_SpellManager_Base_C|GetPlayerPawnRef (Variables|Default|GetSpellManager))))))

(fn AddModifiertoPool
  (params (Modifier :type E_SpellModifiers%20Enum :default "NewEnumerator9") (Spell :type BP%20Spell%20Base%20Object%20Reference))
  (Utilities|Map|Add (Variables|Default|GetModifierSpellPool) Modifier Spell)
  (Variables|BP_SpellBase_C|SetIsModifier Spell true))

(fn TriggerModifier
  (params (ModifierToTrigger :type E_SpellModifiers%20Enum :default "NewEnumerator9") (SpellOwner :type BP%20Spell%20Base%20Object%20Reference))
  (bind (_class _location) (CallFunction|GetModiferSpellClass ModifierToTrigger SpellOwner))
  (bind _spellmanager (Variables|Default|GetSpellManager))
  (bind _modifierspellpool (Variables|Default|GetModifierSpellPool))
  (bind (_value _returnvalue) (Utilities|Map|Find _modifierspellpool ModifierToTrigger))
  (if (Utilities|Enum|Equal(Enum) ModifierToTrigger "NewEnumerator5")
    (if _returnvalue :!label _label
      (LocalVariables|SetNewLocalVar_0 _value)
      (if (Variables|BP_SpellBase_C|GetIsAvailable (LocalVariables|GetNewLocalVar_0))
        _
        (else
          (CallFunction|Reset (LocalVariables|GetNewLocalVar_0) :!label _label_2)))
      (CallFunction|Start (LocalVariables|GetNewLocalVar_0))
      (else
        (bind _returnvalue_2 (Game|SpawnActorfromClass _class (Math|Transform|MakeTransform _location "0, 0, 0" "1,1,1") "AlwaysSpawn" 0 (Variables|Default|GetTarget) (Variables|/Game/_Core/Spells/BP_SpellManager_Base.BP_SpellManager_Base_C|GetSpellTypeInfo _spellmanager) _spellmanager 0))
        (Utilities|IsValid _returnvalue_2
          (:Is%20Valid
            (bind _output_get (LocalVariables|SetNewLocalVar_0 _returnvalue_2))
            (Variables|BP_SpellBase_C|SetIsModifier _output_get true)
            (Variables|BP_SpellBase_C|SetSpellInstigator _output_get self)
            (CallFunction|AddModifiertoPool ModifierToTrigger (LocalVariables|GetNewLocalVar_0))
            (goto _label_2))
          (:Is%20Not%20Valid
            (Development|PrintString "Spell Modifier Not Valid")))))
    (elif (not (Variables|Default|GetIsModifier))
      (goto _label))))

(fn GetModifierSpell
  (params (Modifier :type E_SpellModifiers%20Enum :default "NewEnumerator9"))
  (bind _modifierspellpool (Variables|Default|GetModifierSpellPool))
  (bind (_value _returnvalue) (Utilities|Map|Find _modifierspellpool Modifier))
  (if _returnvalue
    (if (Variables|BP_SpellBase_C|GetIsAvailable _value)
      (return _value true)
      (else
        (return _value false)))
    (else
      (return 0 false))))

(fn GetClosestEnemy
  (return 0))