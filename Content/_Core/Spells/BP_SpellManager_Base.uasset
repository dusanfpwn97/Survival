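; Base spell manager that auto-casts a spell on a cooldown, with an empty CastSpell event as the override point.
; Spell stats load from DT_SpellInfo using a row name derived from the class name.
; CastASpell reuses pooled spell actors round-robin, spawning and pooling a new one when the checked slot is busy or missing.
; Compatible modifiers are stored per inventory slot, returning replaced ones to the player and refreshing the HUD.
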(event Custom|AddSpellModifier
  (params (InventoryIndex :type Integer) (SpellModifier :type E_SpellModifiers%20Enum :default "NewEnumerator0"))
  (bind _currentmodifiers (Variables|Default|GetCurrentModifiers))
  (bind (_value _returnvalue) (Utilities|Map|Find _currentmodifiers InventoryIndex))
  (if (CallFunction|CanModifySpell SpellModifier)
    (if _returnvalue
      (Utilities|FlowControl|Sequence
        (:then_0
          (Development|PrintString (Utilities|String|Append (Utilities|String|EnumtoString SpellModifier) " Modifier already exists at this slot. Replacing..." (Utilities|GetDisplayName self)) true true "(R=1.000000,G=0.750000,B=0.000000,A=1.000000)" 3.0)
          (bind _asbp_player (Utilities|Casting|CastToBP_Player (Game|Player|GetPlayerPawn 0)))
          (Default|AddModifiertoInventory _asbp_player _value))
        (:then_1
          (Utilities|Map|Add (Variables|Default|GetCurrentModifiers) InventoryIndex SpellModifier :!label _label)
          (Class|BPHUDInterface|RefreshInventory(Message) (HUD|GetHUD (Game|GetPlayerController 0)))))
      (else
        (goto _label)))))

(event Custom|UpdateManager
  (if (<= (- (Variables|Default|GetCurrentCooldown) (Utilities|Time|GetWorldDeltaSeconds)) 0.0)
    (Variables|Default|SetCurrentCooldown (.cooldown (Variables|Default|GetSpellTypeInfo)))
    (CallFunction|CastSpell)
    (else
      (Variables|Default|SetCurrentCooldown (- (Variables|Default|GetCurrentCooldown) (Utilities|Time|GetWorldDeltaSeconds))))))

(event Custom|CastSpell)

(event EventBeginPlay
  (CallFunction|InitSpellType))

(event EventTick
  (params (DeltaSeconds :type Float%20%28single-precision%29))
  (CallFunction|UpdateManager))

(event EventOnModifiedSpell
  (params (Spell :type BP%20Spell%20Manager%20Base%20Object%20Reference) (UpgradeUsed :type BP%20Drop%20Base%20Object%20Reference) (InventoryIndex :type Integer))
  (CallFunction|AddSpellModifier InventoryIndex (Variables|/Game/_Core/Drop/BP_DropBase.BP_DropBase_C|GetSpellModifier UpgradeUsed)))

(fn CanModifySpell
  (params (SpellModifier :type E_SpellModifiers%20Enum :default "NewEnumerator9"))
  (if (Utilities|Enum|NotEqual(Enum) SpellModifier "NewEnumerator9")
    (if (Utilities|Array|ContainsItem (.compatiblemodifiers (Variables|Default|GetSpellTypeInfo)) SpellModifier)
      (return true)
      (else
        (Development|PrintString (Utilities|String|Append (Utilities|String|EnumtoString SpellModifier) " not compatible with " (Utilities|String|EnumtoString (Utilities|Array|Get(acopy) (.requiredcasttypes (Variables|Default|GetSpellTypeInfo)))) "! " (Utilities|GetDisplayName self)) true true "(R=1.000000,G=0.182798,B=0.000000,A=1.000000)" 5.0)
        (return false)))
    (else
      (Development|PrintString "Spell modifier null. BP_BaseSpellManager->CanModifySpell")
      (return false))))

(fn InitSpellType
  (bind _self self)
  (bind _returnvalue (Utilities|GetClass _self))
  (bind _spellname (CallFunction|GetSpellNamefromClassName _returnvalue))
  (bind _returnvalue_2 (Utilities|GetDataTableRow "/Game/GameSettings/DT_SpellInfo.DT_SpellInfo" _spellname)
    (:then
      (Variables|Default|SetSpellTypeInfo _returnvalue_2))
    (:RowNotFound
      (Development|PrintString (Utilities|String|Append "Spell NOT FOUND! BP_SM_Base->InitSpellType - " (Utilities|String|ToString(Name) _spellname)) true true "(R=1.000000,G=0.002236,B=0.000000,A=1.000000)" 255.0))))

(fn CastASpell
  (params (SpellToCast :type BP%20Spell%20Base%20Class%20Reference) (Location :type Vector))
  (bind _pooledspells (Variables|Default|GetPooledSpells))
  (bind _pooledspells_2 (Variables|Default|GetPooledSpells))
  (bind _returnvalue (Utilities|Array|Length _pooledspells_2))
  (bind _output (Utilities|Array|Get(acopy) _pooledspells))
  (if (>= (- _returnvalue 1) (+ (Variables|Default|GetLastCastSpellIndex) 1))
    (if (Variables|/Game/_Core/Spells/BP_SpellBase.BP_SpellBase_C|GetIsAvailable (Utilities|Array|Get(acopy) _pooledspells_2 (+ (Variables|Default|GetLastCastSpellIndex) 1)))
      (LocalVariables|SetTempSpellThatHasBeenCast (Utilities|Array|Get(acopy) (Variables|Default|GetPooledSpells) (+ (Variables|Default|GetLastCastSpellIndex) 1)))
      (Variables|Default|SetLastCastSpellIndex (+ (Variables|Default|GetLastCastSpellIndex) 1))
      (else
        (bind _returnvalue_2 (Game|SpawnActorfromClass SpellToCast (Math|Transform|MakeTransform Location "0, 0, 0" "1,1,1") "Undefined" 0 (Variables|Default|GetTarget) (Variables|Default|GetSpellTypeInfo) self 0 :!label _label))
        (bind _output_get (LocalVariables|SetTempSpellThatHasBeenCast _returnvalue_2))
        (bind _index (CallFunction|AddSpelltoPool _output_get))
        (Variables|Default|SetLastCastSpellIndex _index)))
    (elif (> _returnvalue 0)
      (if (Variables|/Game/_Core/Spells/BP_SpellBase.BP_SpellBase_C|GetIsAvailable _output)
        (LocalVariables|SetTempSpellThatHasBeenCast _output)
        (Variables|Default|SetLastCastSpellIndex 0)
        (else
          (goto _label)))
      (else
        (goto _label))))
  (Default|Start (LocalVariables|GetTempSpellThatHasBeenCast) (Variables|Default|GetTarget) Location)
  (return (LocalVariables|GetTempSpellThatHasBeenCast)))

(fn AddSpelltoPool
  (params (Spell :type BP%20Spell%20Base%20Object%20Reference%20%28by%20ref%29))
  (bind _returnvalue (Utilities|Array|Add (Variables|Default|GetPooledSpells) Spell))
  (bind _output_get (Variables|/Game/_Core/Spells/BP_SpellBase.BP_SpellBase_C|SetPoolIndex Spell _returnvalue))
  (return _output_get))

(fn GetSpellsinInventory
  (return 0))

(fn GetUpgradesinInventory
  (params (SpecificUpgrade :type E_AllUpgradeTypes%20Enum :default "NewEnumerator5"))
  (return 0))