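; Base actor Blueprint for spells, providing the shared lifecycle that child spells build on.
; On BeginPlay it calls Restart, which caches a valid Target's location and the normalized direction toward it, then Init, an empty hook for child setup.
; The construction script also runs Init, but only on Windows.
; Stop and the lookup functions for cast types, modifiers, passive upgrades and closest enemy are empty here.
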(event Custom|Restart
  (bind _target (Variables|Default|GetTarget))
  (Utilities|IsValid _target
    (:Is%20Valid
      (Variables|Default|SetStartingTargetLocation (Transformation|GetActorLocation _target))
      (Variables|Default|SetStartingDirection (Math|Vector|Normalize (- (Variables|Default|GetStartingTargetLocation) (Transformation|GetActorLocation)))))))

(event Custom|Stop)

(event Custom|Init)

(event EventBeginPlay
  (CallFunction|Restart)
  (CallFunction|Init))

(event Collision|EventActorBeginOverlap
  (params (OtherActor :type Actor%20Object%20Reference)))

(event EventTick
  (params (DeltaSeconds :type Float%20%28single-precision%29)))

(fn ConstructionScript
  (if (Utilities|Enum|Equal(Enum) (Game|GetPlatformName) "Windows")
    (CallFunction|Init)))

(fn GetCastTypeInfo
  (params (CastType :type E_SpellCastType%20Enum :default "NewEnumerator8"))
  (return ""))

(fn GetClosestEnemy
  (return 0))

(fn GetCompatiblesforCastType
  (params (CastType :type E_SpellCastType%20Enum :default "NewEnumerator8"))
  (return "NewEnumerator9" "NewEnumerator9"))

(fn GetSpellModifierInfo
  (params (SpellModifier :type E_SpellModifiers%20Enum :default "NewEnumerator9"))
  (return ""))

(fn GetSpellPassiveUpgradeInfo
  (params (SpellPassiveUpgrade :type E_SpellPassives%20Enum :default "NewEnumerator9"))
  (return ""))