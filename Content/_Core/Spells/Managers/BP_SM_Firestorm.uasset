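; Spell manager for Firestorm, which spawns a projectile high above the area around the player on each cast.
; CastSpell runs the parent logic, then spawns one BP_FirestormProjectile at a random circumference point around the player pawn, using a randomized radius and a fixed world height.
; The projectile receives the current Target and a reference back to this manager.
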(event EventBeginPlay
  (|CallParentFunction) ; This node is disabled and will not be called.\nDrag off pins to build functionality.
)

(event EventTick
  (params (DeltaSeconds :type Float%20%28single-precision%29))
  (|CallParentFunction DeltaSeconds) ; This node is disabled and will not be called.\nDrag off pins to build functionality.
)

(event EventCastSpell
  (bind _returnvalue (Math|Random|RandomFloat))
  (bind _playerpawnref (Variables|Default|GetPlayerPawnRef))
  (bind _returnvalue_2 (Transformation|GetActorLocation _playerpawnref))
  (bind _returnvalue_3 (* _returnvalue 1e+03))
  (bind _pointlocation (CallFunction|GetRandomPointinCircumference _returnvalue_3 _returnvalue_2))
  (|CallParentFunction)
  (Game|SpawnActorfromClass "/Game/_Core/Spells/Spells/BP_FirestormProjectile.BP_FirestormProjectile_C" (Math|Transform|MakeTransform (Math|Vector|MakeVector (.x _pointlocation) (.y _pointlocation) 2e+03) "0, 0, 0" "1,1,1") "Undefined" 0 (Variables|Default|GetTarget) self 0))