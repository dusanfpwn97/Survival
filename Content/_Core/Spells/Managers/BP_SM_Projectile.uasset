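; BP_SM_Projectile is a spell manager for projectile spells, currently a stub whose CastSpell_1 event does nothing.
; Disconnected nodes hold projectile logic that never runs: a class-checked PrepareSpell at the player's SpellStart, with an error print for invalid classes.
; Other orphaned nodes query the closest enemy and, given a modifier, cast again after an eighth of the spell's cooldown.
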(event Custom|CastSpell_1
  (params (Target :type Actor%20Object%20Reference) (IsModifier :type Boolean) (BaseLocationObject :type Scene%20Component%20Object%20Reference)))

(event EventBeginPlay
  (|CallParentFunction) ; This node is disabled and will not be called.\nDrag off pins to build functionality.
)

(event EventTick
  (params (DeltaSeconds :type Float%20%28single-precision%29))
  (|CallParentFunction DeltaSeconds) ; This node is disabled and will not be called.\nDrag off pins to build functionality.
)