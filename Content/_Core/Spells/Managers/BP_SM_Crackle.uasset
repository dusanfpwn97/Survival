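; Spell manager for the Crackle spell, which casts at the enemy closest to the player.
; CastSpell runs the parent logic, then asks the player pawn for its closest enemy.
; If one is valid, it spawns BP_SpellCrackle slightly offset from the player toward that enemy, using only the X and Y of that point.
; The spawned spell receives the target, the spell type info and a reference to this manager.
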(event EventBeginPlay
  (|CallParentFunction) ; This node is disabled and will not be called.\nDrag off pins to build functionality.
)

(event EventTick
  (params (DeltaSeconds :type Float%20%28single-precision%29))
  (|CallParentFunction DeltaSeconds) ; This node is disabled and will not be called.\nDrag off pins to build functionality.
)

(event EventCastSpell
  (bind _returnvalue (Game|Player|GetPlayerPawn 0))
  (|CallParentFunction)
  (bind _enemy (Class|BPCombatInterface|GetClosestEnemy(Message) _returnvalue))
  (bind _output_get (Variables|Default|SetTarget _enemy))
  (Utilities|IsValid _output_get
    (:Is%20Valid
      (Game|SpawnActorfromClass "/Game/_Core/Spells/Spells/BP_SpellCrackle.BP_SpellCrackle_C" (Math|Transform|MakeTransform (Math|Vector|MakeVector (.x (+ (* (Math|Vector|GetForwardVector (Math|Rotator|FindLookatRotation (Transformation|GetActorLocation _returnvalue) (Transformation|GetActorLocation (Variables|Default|GetTarget)))) 3e+01) (Transformation|GetActorLocation (Game|Player|GetPlayerPawn 0)))) (.y (+ (* (Math|Vector|GetForwardVector (Math|Rotator|FindLookatRotation (Transformation|GetActorLocation _returnvalue) (Transformation|GetActorLocation (Variables|Default|GetTarget)))) 3e+01) (Transformation|GetActorLocation (Game|Player|GetPlayerPawn 0)))) 0.0) "0, 0, 0" "1,1,1") "Undefined" 0 (Variables|Default|GetTarget) (Variables|Default|GetSpellTypeInfo) self 0))))