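; Blueprint helper functions for random circle points, nearest-actor lookup and spell naming.
; The point helper picks a random angle on an XY circle around an offset, adding the offset's Z twice.
; The actor search loops through valid entries, tracking the smallest distance to a reference actor.
; The spell name comes from trimming two trailing and six leading characters off a spell manager's class display name.
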(fn GetRandomPointinCircumference
  (params (Radius :type Float%20%28single-precision%29) (Offset :type Vector))
  (LocalVariables|SetL_Radius Radius)
  (LocalVariables|SetL_Offset Offset)
  (LocalVariables|SetRandomAngle (* (Math|Random|RandomFloat) 3.1415 2.0))
  (return (+ (LocalVariables|GetL_Offset) (Math|Vector|MakeVector (* (Math|Trig|Cos(Radians) (LocalVariables|GetRandomAngle)) (LocalVariables|GetL_Radius)) (* (Math|Trig|Sin(Radians) (LocalVariables|GetRandomAngle)) (LocalVariables|GetL_Radius)) (.Z (Math|Vector|BreakVector (LocalVariables|GetL_Offset)))))))

(fn GetClosestActor
  (params (ActorsToCheck :type Array%20of%20Actor%20Object%20References) (ReferenceActor :type Actor%20Object%20Reference))
  (if (> (Utilities|Array|Length ActorsToCheck) 0)
    (for (_array_element _array_index) ActorsToCheck
      (Utilities|IsValid _array_element
        (:Is%20Valid
          (if (< (Transformation|GetDistanceTo _array_element ReferenceActor) (LocalVariables|GetClosestLocation))
            (LocalVariables|SetClosestLocation (Transformation|GetDistanceTo _array_element ReferenceActor))
            (LocalVariables|SetIndexOfClosestActor _array_index)))))
    (return (Utilities|Array|Get(acopy) ActorsToCheck (LocalVariables|GetIndexOfClosestActor)))
    (else
      (return 0))))

(fn GetSpellNamefromClassName
  (params (SpellManagerClass :type BP%20Spell%20Manager%20Base%20Class%20Reference))
  (return (Utilities|String|StringToName (Utilities|String|RightChop (Utilities|String|LeftChop (Utilities|GetClassDisplayName SpellManagerClass) 2) 6))))