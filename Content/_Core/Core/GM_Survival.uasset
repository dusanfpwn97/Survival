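; Survival game mode that continuously spawns enemies around the player and relays music beats to them and the player pawn.
; BeginPlay spawns BP_MusicPlayer and starts a fast looping timer that adds BP_EnemyNormal at randomized positions based on SpawnRadius around the player.
; Spawned enemies are tracked in an array, which OnBeat walks to notify each valid one before messaging the player; the array is never pruned here.
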(event Custom|SpawnEnemies
  (CallFunction|SpawnEnemy "/Game/_Core/Enemies/BP_EnemyNormal.BP_EnemyNormal_C"))

(event EventBeginPlay
  (Utilities|Time|SetTimerbyEvent (delegate Custom|SpawnEnemies) 0.35 true)
  (Game|SpawnActorfromClass "/Game/_Core/Music/BP_MusicPlayer.BP_MusicPlayer_C" (Math|Transform|MakeTransform (Transformation|GetActorLocation) "0, 0, 0" "1,1,1") "Undefined" 0 0))

(event EventOnBeat
  (for _array_element (Variables|Default|GetSpawnedEnemies)
    (Utilities|IsValid _array_element
      (:Is%20Valid
        (Default|OnBeat _array_element))))
  (Class|BPMusicEventsBroadcaster|OnBeat(Message) (Game|Player|GetPlayerPawn 0)))

(fn ConstructionScript)

(fn SpawnEnemy
  (params (EnemyClass :type BP%20Enemy%20Base%20Class%20Reference))
  (bind _returnvalue (Game|Player|GetPlayerPawn 0))
  (bind _spawnradius (Variables|Default|GetSpawnRadius))
  (bind _returnvalue_2 (Transformation|GetActorLocation _returnvalue))
  (bind _pointlocation (CallFunction|GetRandomPointinCircumference _spawnradius _returnvalue_2))
  (bind (_x _y) (Math|Vector|BreakVector _pointlocation))
  (bind _returnvalue_3 (Game|SpawnActorfromClass EnemyClass (Math|Transform|MakeTransform (Math|Vector|MakeVector _x _y 5e+01) "0, 0, 0" "1,1,1") "Undefined" 0 0))
  (Utilities|Array|Add (Variables|Default|GetSpawnedEnemies) _returnvalue_3))