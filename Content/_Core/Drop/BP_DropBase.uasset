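; Base Blueprint for drops that carry a spell upgrade, categorised as cast type, spell modifier or passive upgrade.
; On BeginPlay it runs ErrorCheck, which switches on UpgradeType and verifies the two fields of the other categories hold their expected enum values.
; A mismatch prints a long-lived red setup error naming the actor.
; No overlap, pickup or tick logic is implemented here.
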(event EventBeginPlay
  (CallFunction|ErrorCheck))

(event Collision|EventActorBeginOverlap
  (params (OtherActor :type Actor%20Object%20Reference)))

(event EventTick
  (params (DeltaSeconds :type Float%20%28single-precision%29)))

(fn ConstructionScript)

(fn ErrorCheck
  (switch Utilities|FlowControl|Switch|SwitchonE_AllUpgradeTypes (Variables|Default|GetUpgradeType)
    (:NewEnumerator2
      (if (or (Utilities|Enum|NotEqual(Enum) (Variables|Default|GetSpellModifier) "NewEnumerator9") (Utilities|Enum|NotEqual(Enum) (Variables|Default|GetPassiveUpgrade) "NewEnumerator9"))
        (Development|PrintString (Utilities|String|Append "Setup error in " (Utilities|GetDisplayName self) "!") true true "(R=1.000000,G=0.000000,B=0.014919,A=1.000000)" 2e+01 :!label _label)))
    (:NewEnumerator3
      (if (or (Utilities|Enum|NotEqual(Enum) (Variables|Default|GetSpellCastType) "NewEnumerator8") (Utilities|Enum|NotEqual(Enum) (Variables|Default|GetPassiveUpgrade) "NewEnumerator9"))
        (goto _label)))
    (:NewEnumerator4
      (if (or (Utilities|Enum|NotEqual(Enum) (Variables|Default|GetSpellCastType) "NewEnumerator8") (Utilities|Enum|NotEqual(Enum) (Variables|Default|GetSpellModifier) "NewEnumerator9"))
        (goto _label)))))