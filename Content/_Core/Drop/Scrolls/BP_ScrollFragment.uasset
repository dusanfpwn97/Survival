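; BP_ScrollFragment is a scroll fragment drop actor that animates itself in the world with a spin and a bob.
; Each Tick it yaws at a constant rate scaled by delta time and adds a sine-of-game-time vertical offset.
; The bob offset is not scaled by delta time, so its height varies with frame rate.
; The graph holds no pickup logic of its own, and SpinCounter is unused.
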(event EventBeginPlay
  (|CallParentFunction) ; This node is disabled and will not be called.\nDrag off pins to build functionality.
)

(event Collision|EventActorBeginOverlap
  (params (OtherActor :type Actor%20Object%20Reference))
  (|CallParentFunction OtherActor) ; This node is disabled and will not be called.\nDrag off pins to build functionality.
)

(event EventTick
  (params (DeltaSeconds :type Float%20%28single-precision%29))
  (|CallParentFunction DeltaSeconds)
  (Class|Actor|AddActorWorldRotation (Math|Rotator|MakeRotator 0.0 0.0 (* DeltaSeconds 5e+01)))
  (Transformation|AddActorWorldOffset (Math|Vector|MakeVector 0.0 0.0 (* (Math|Trig|Sin(Radians) (* (Utilities|Time|GetTimeSeconds) 4.0)) 1.0))))

(fn ConstructionScript
  (|CallParentFunction))