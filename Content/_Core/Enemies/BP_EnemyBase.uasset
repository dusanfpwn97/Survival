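; Base enemy actor that moves straight toward the player pawn every tick, without sweep, while alive.
; On BeginPlay it loads speed and health from DT_EnemyStats, deriving the row name from its trimmed class name.
; Spell hits subtract health, briefly swap to a damage material, and trigger death once at zero, clearing the alive flag.
; Reset only restores that flag; GetClosestEnemy and OnBeat are empty stubs.
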(event Custom|Die
  (Variables|Default|SetIsAlive false))

(event Custom|Reset
  (Variables|Default|SetIsAlive true))

(event Custom|OnReceivedDamageVisual
  (Rendering|Material|SetMaterial (Variables|Default|GetStaticMesh) 0 "/Game/Characters/Test_enemy/M_EnemyDamageMat.M_EnemyDamageMat")
  (Utilities|FlowControl|RetriggerableDelay 0.1)
  (Rendering|Material|SetMaterial (Variables|Default|GetStaticMesh) 0 (Variables|Default|GetStartingMat)))

(event Custom|PaintDebug
  (Rendering|Material|SetMaterial (Variables|Default|GetStaticMesh) 0 "/Game/Characters/Test_enemy/M_Debug.M_Debug"))

(event EventBeginPlay
  (Variables|Default|SetTargetActor (Game|Player|GetPlayerPawn 0))
  (CallFunction|SetStats)
  (Variables|Default|SetStartingMat (Rendering|Material|GetMaterial (Variables|Default|GetStaticMesh) 0)))

(event EventOnDamaged
  (params (Spell :type BP%20Spell%20Base%20Object%20Reference))
  (bind _output_get (Variables|Default|SetHealth (- (Variables|Default|GetHealth) (.damage (Variables|/Game/_Core/Spells/BP_SpellManager_Base.BP_SpellManager_Base_C|GetSpellTypeInfo (Variables|/Game/_Core/Spells/BP_SpellBase.BP_SpellBase_C|GetSpellManager Spell))))))
  (CallFunction|OnReceivedDamageVisual)
  (if (<= _output_get 0.0)
    (Utilities|FlowControl|DoOnce false
      (:Completed
        (CallFunction|Die)))))

(event EventTick
  (params (DeltaSeconds :type Float%20%28single-precision%29))
  (bind _targetactor (Variables|Default|GetTargetActor))
  (Utilities|IsValid _targetactor
    (:Is%20Valid
      (if (Variables|Default|GetIsAlive)
        (Transformation|AddActorWorldOffset (* (* (Math|Vector|Normalize (- (Transformation|GetActorLocation _targetactor) (Transformation|GetActorLocation))) DeltaSeconds) (Variables|Default|GetSpeed)))))))

(fn ConstructionScript)

(fn SetStats
  (bind _returnvalue (Utilities|GetDataTableRow "/Game/GameSettings/DT_EnemyStats.DT_EnemyStats" (Utilities|String|StringToName (Utilities|String|LeftChop (Utilities|GetClassDisplayName (Utilities|GetClass self)) 2)))
    (:then
      (Variables|Default|SetInitialStats _returnvalue)
      (Variables|Default|SetSpeed (.speed (Variables|Default|GetInitialStats)))
      (Variables|Default|SetHealth (.health (Variables|Default|GetInitialStats))))
    (:RowNotFound
      (Development|PrintString (Utilities|String|Append "Data table row now found! " (Utilities|GetDisplayName self)) true true "(R=1.000000,G=0.000000,B=0.055031,A=1.000000)" 5.0))))

(fn GetClosestEnemy
  (return 0))

(fn GetIsAlive
  (return (Variables|Default|GetIsAlive)))

(fn OnBeat
  (return))