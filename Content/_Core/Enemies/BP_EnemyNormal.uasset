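; BP_EnemyNormal is the normal enemy Blueprint, which animates the scale of its mesh to a beat.
; Each OnBeat event restarts a timeline from the start, whose track value is converted to a vector and applied as the StaticMesh world scale.
; BeginPlay and the construction script only call the parent, and Tick and overlap events are disabled, so this graph adds only the beat-driven scaling.
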(event EventBeginPlay
  (|CallParentFunction))

(event Collision|EventActorBeginOverlap
  (params (OtherActor :type Actor%20Object%20Reference))
  (|CallParentFunction OtherActor) ; This node is disabled and will not be called.\nDrag off pins to build functionality.
)

(event EventTick
  (params (DeltaSeconds :type Float%20%28single-precision%29))
  (|CallParentFunction DeltaSeconds) ; This node is disabled and will not be called.\nDrag off pins to build functionality.
)

(event EventOnBeat
  (bind _newtrack_0 (Timeline|Timeline_0 PlayFromStart)
    (:Update
      (Transformation|SetWorldScale3D (Variables|Default|GetStaticMesh) (Math|Conversions|ToVector(Float) _newtrack_0)))))

(fn ConstructionScript
  (|CallParentFunction))