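; BP_GI, apparently the Game Instance, serves as a lookup point for spell-crafting data: cast types, spell modifiers and passive upgrades.
; Getter functions look up enum keys in info maps and print an on-screen error when an entry is missing.
; GetCompatiblesForCastType pulls the compatible modifiers and passive upgrades from a cast type's entry.
; GetInventoryInfo and the Shutdown event are empty stubs.
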(event EventShutdown)

(fn GetCastTypeInfo
  (params (CastType :type E_SpellCastType%20Enum :default "NewEnumerator8"))
  (bind _casttypeinfo (Variables|Default|GetCastTypeInfo))
  (bind (_value _returnvalue) (Utilities|Map|Find _casttypeinfo CastType))
  (if _returnvalue
    (return _value)
    (else
      (Development|PrintString (Utilities|String|Append (Utilities|String|EnumtoString CastType) " NOT FOUND!") true true "(R=1.000000,G=0.036913,B=0.000000,A=1.000000)" 5.0))))

(fn GetCompatiblesforCastType
  (params (CastType :type E_SpellCastType%20Enum :default "NewEnumerator8"))
  (bind _casttypeinfo (Variables|Default|GetCastTypeInfo))
  (bind (_value _returnvalue) (Utilities|Map|Find _casttypeinfo CastType))
  (if _returnvalue
    (return (.compatiblespellmodifiers _value) (.compatiblepassiveupgrades _value))
    (else
      (Development|PrintString "No compatible Modifiers Found! Should not happen!" true true "(R=1.000000,G=0.044963,B=0.000000,A=1.000000)" 5.0))))

(fn GetInventoryInfo
  (return 0 0 0))

(fn GetSpellModifierInfo
  (params (SpellModifier :type E_SpellModifiers%20Enum :default "NewEnumerator9"))
  (bind _spellmodifierinfo (Variables|Default|GetSpellModifierInfo))
  (bind (_value _returnvalue) (Utilities|Map|Find _spellmodifierinfo SpellModifier))
  (if _returnvalue
    (return _value)
    (else
      (Development|PrintString (Utilities|String|Append (Utilities|String|EnumtoString SpellModifier) " NOT FOUND!") true true "(R=1.000000,G=0.036913,B=0.000000,A=1.000000)" 5.0))))

(fn GetSpellPassiveUpgradeInfo
  (params (SpellPassiveUpgrade :type E_SpellPassives%20Enum :default "NewEnumerator9"))
  (bind _spellpassiveupgradeinfo (Variables|Default|GetSpellPassiveUpgradeInfo))
  (bind (_value _returnvalue) (Utilities|Map|Find _spellpassiveupgradeinfo SpellPassiveUpgrade))
  (if _returnvalue
    (return _value)
    (else
      (Development|PrintString (Utilities|String|Append (Utilities|String|EnumtoString SpellPassiveUpgrade) " NOT FOUND!") true true "(R=1.000000,G=0.036913,B=0.000000,A=1.000000)" 5.0))))